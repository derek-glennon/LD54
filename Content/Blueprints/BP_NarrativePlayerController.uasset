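; Player controller for a narrative game where clicks talk to characters, use pillars, or capture characters.
; It creates capture, dialogue and fade widgets, passing the dialogue widget to interactable actors.
; In capture mode, a cursor trace sends characters to free BP_CapturedLocation slots within a size limit; clicking captured ones releases them.
; The ending room releases captives with staggered fades before its dialogue, and a reset event restores the loop.
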(event Custom|ToCaptureMode
  (Variables|Capture|SetInCaptureMode true)
  (Variables|Default|SetCurrentMouseCursor "GrabHandClosed"))

(event Custom|OnEndingRoomArrived
  (Variables|Ending|SetInEndingRoom true)
  (Input|DisableInput 0)
  (for _array_element (Actor|GetAttachedActors (Variables|Default|GetCurrentRoom) true false)
    (bind _asbp_narrative_character (Utilities|Casting|CastToBP_NarrativeCharacter _array_element))
    (Variables|Ending|SetEndingDialogue _asbp_narrative_character)
    (Utilities|FlowControl|Delay 1.0)
    (bind _outactors (Actor|GetAllActorsOfClass "/Game/Characters/BP_NarrativeCharacter.BP_NarrativeCharacter_C"))
    (for _array_element_2 _outactors
      (if (Variables|/Game/Characters/BP_NarrativeCharacter.BP_NarrativeCharacter_C|GetIsCaptured _array_element_2)
        (Utilities|Array|Add (Variables|Capture|GetCapturedCharacters) _array_element_2)))
    (for (_array_element_3 _array_index) (Variables|Capture|GetCapturedCharacters)
      (Variables|/Game/Characters/BP_NarrativeCharacter.BP_NarrativeCharacter_C|SetRoomTransform _array_element_3 (Math|Transform|MakeRelativeTransform (Math|Transform|MakeTransform "0.000000,0.000000,200.000000") (Transformation|GetActorTransform (Variables|Default|GetCurrentRoom))))
      (Default|OnRelease _array_element_3 (* _array_index 1.5))
      (Default|FadeOut _array_element_3 (* _array_index 1.5)))
    (Utilities|FlowControl|Delay 2.0)
    (Class|BPIInteractableObject|OnInteract(Message) (Variables|Ending|GetEndingDialogue))))

(event Custom|ResetGameLoop
  (Variables|Capture|SetInCaptureMode false)
  (Variables|Capture|SetCurrentCapturedAmount 0)
  (Default|OnCaptureSpaceLeftChanged (Variables|Capture|GetCaptureWidget) (Variables|Capture|GetCaptureSizeLimit))
  (Default|CaptureLimitReleased (Variables|Capture|GetCaptureWidget))
  (Default|ResetDialogue (Variables|Default|GetDialogueWidget))
  (Utilities|Array|Clear (Variables|Capture|GetCapturedCharacters))
  (Variables|Ending|SetInEndingRoom false)
  (for _array_element (Actor|GetAttachedActors (Variables|Default|GetCurrentRoom) true false)
    (bind _asbp_pillar (Utilities|Casting|CastToBP_Pillar _array_element))
    (Default|OnInteract _asbp_pillar))
  (Utilities|FlowControl|Delay 3.0)
  (bind _outactors (Actor|GetAllActorsOfClass "/Game/Characters/BP_NarrativeCharacter.BP_NarrativeCharacter_C"))
  (for _array_element_2 _outactors
    (bind _asbp_narrative_character (Utilities|Casting|CastToBP_NarrativeCharacter _array_element_2))
    (Default|ResetCharacter _asbp_narrative_character))
  (Default|ResetCharacter (Variables|Ending|GetEndingDialogue))
  (for _array_element_3 (Variables|Default|GetCapturedLocations)
    (Variables|/Game/Blueprints/BP_CapturedLocation.BP_CapturedLocation_C|SetIsOccupied _array_element_3 false))
  (Default|ToGame (Variables|Ending|GetFadeScreen)))

(event Input|EnhancedActionEvents|EnhancedInputActionIA_Click
  (params (ActionValue :type Boolean) (ElapsedSeconds :type Float%20%28double-precision%29) (TriggeredSeconds :type Float%20%28double-precision%29) (InputAction :type Input%20Action%20Object%20Reference :default "/Game/Input/IA_Click.IA_Click"))
  (bind _hitresult (Game|Player|GetHitResultUnderCursorbyChannel "TraceTypeQuery1" true))
  (bind (_bblockinghit _binitialoverlap _time _distance _location _impactpoint _normal _impactnormal _physmat _hitactor) (Collision|BreakHitResult _hitresult))
  (:Canceled
    (if _bblockinghit :!label _label
      (Variables|Default|SetClickLocation _location)
      (bind _output_get (Variables|Default|SetClickActor _hitactor))
      (if (Utilities|DoesObjectImplementInterface _output_get "/Game/Blueprints/Interfaces/BPI_InteractableObject.BPI_InteractableObject_C")
        (bind _asbp_narrative_character (Utilities|Casting|CastToBP_NarrativeCharacter (Variables|Default|GetClickActor))
          (:then
            (Variables|Capture|SetCaptureNarrativeCharacter _asbp_narrative_character)
            (if (Variables|Capture|GetInCaptureMode)
              ;[0.3036 1 0.3575] Capture Narrative Character
              (if (not (Variables|/Game/Characters/BP_NarrativeCharacter.BP_NarrativeCharacter_C|GetIsCaptured (Variables|Capture|GetCaptureNarrativeCharacter))) ; Make sure you are not tring to capture \nsomething that is already captured
                (if (<= (+ (Variables|Capture|GetCurrentCapturedAmount) (Variables|/Game/Characters/BP_NarrativeCharacter.BP_NarrativeCharacter_C|GetCaptureSize (Variables|Capture|GetCaptureNarrativeCharacter))) (Variables|Capture|GetCaptureSizeLimit)) ; Can the thing you are trying to capture fit?
                  (bind _output_get_2 (Variables|Capture|SetCurrentCapturedAmount (+ (Variables|Capture|GetCurrentCapturedAmount) (Variables|/Game/Characters/BP_NarrativeCharacter.BP_NarrativeCharacter_C|GetCaptureSize (Variables|Capture|GetCaptureNarrativeCharacter)))))
                  (Default|OnCaptureSpaceLeftChanged (Variables|Capture|GetCaptureWidget) (- (Variables|Capture|GetCaptureSizeLimit) _output_get_2))
                  (bind _goalcapturedlocation (CallFunction|FindAvailableCaptureLocation))
                  (Class|BPIInteractableObject|OnCapture(Message) (Variables|Capture|GetCaptureNarrativeCharacter) _goalcapturedlocation)
                  (if (== (Variables|Capture|GetCurrentCapturedAmount) (Variables|Capture|GetCaptureSizeLimit)) ; Check limit
                    (Default|CaptureLimitReached (Variables|Capture|GetCaptureWidget)))
                  ;[0.3036 1 0.3575] Leave Capture Mode Once You Capture Something
                  (Variables|Capture|SetInCaptureMode false)
                  (Variables|Default|SetCurrentMouseCursor "Default")
                  (else
                    (Variables|Default|SetCurrentMouseCursor "SlashedCircle")
                    (Utilities|FlowControl|Delay 2.0)
                    (Variables|Default|SetCurrentMouseCursor "GrabHandClosed")))
                (else
                  ;[0.3036 1 0.3575] Release Captured Narrative Character
                  (if (== (Variables|Capture|GetCurrentCapturedAmount) (Variables|Capture|GetCaptureSizeLimit)) :!label _label_2
                    (Default|CaptureLimitReleased (Variables|Capture|GetCaptureWidget)))
                  (bind _output_get_3 (Variables|Capture|SetCurrentCapturedAmount (- (Variables|Capture|GetCurrentCapturedAmount) (Variables|/Game/Characters/BP_NarrativeCharacter.BP_NarrativeCharacter_C|GetCaptureSize (Variables|Capture|GetCaptureNarrativeCharacter)))))
                  (Default|OnCaptureSpaceLeftChanged (Variables|Capture|GetCaptureWidget) (- (Variables|Capture|GetCaptureSizeLimit) _output_get_3))
                  (CallFunction|ReleaseCaptureLocation (Variables|/Game/Characters/BP_NarrativeCharacter.BP_NarrativeCharacter_C|GetCapturedLocation (Variables|Capture|GetCaptureNarrativeCharacter)))
                  (Default|OnRelease (Variables|Capture|GetCaptureNarrativeCharacter) 0.0)
                  ;[0.3036 1 0.3575] If you were in capture mode, leave it
                  (if (Variables|Capture|GetInCaptureMode)
                    (Variables|Capture|SetInCaptureMode false)
                    (Variables|Default|SetCurrentMouseCursor "Default"))))
              (elif (Variables|/Game/Characters/BP_NarrativeCharacter.BP_NarrativeCharacter_C|GetIsCaptured (Variables|Capture|GetCaptureNarrativeCharacter))
                (goto _label_2)
                (else
                  (Class|BPIInteractableObject|OnInteract(Message) (Variables|Capture|GetCaptureNarrativeCharacter))))))
          (:CastFailed
            (Class|BPIInteractableObject|OnInteract(Message) (Variables|Default|GetClickActor)) ; Pillars
          ))
        (else
          (Class|BPIInteractableObject|OnClickAway(Message) (Variables|Default|GetDialogueWidget))
          ;[0.3036 1 0.3575] Leave Capture Mode
          (if (Variables|Capture|GetInCaptureMode)
            (Variables|Capture|SetInCaptureMode false)
            (Variables|Default|SetCurrentMouseCursor "Default"))))))
  (:Completed
    (goto _label)))

(event EventBeginPlay
  (bind _returnvalue (PlayerController|LocalPlayerSubsystems|GetEnhancedInputLocalPlayerSubsystem))
  ;[1 0.923 0.03199] Add Mapping Context
  (Utilities|IsValid _returnvalue
    (:Is%20Valid
      (Input|AddMappingContext _returnvalue "/Game/Input/IMC_Default_Narrative.IMC_Default_Narrative" 0 "(bIgnoreAllPressedKeysUntilRelease=True,bForceImmediately=False)")
      ;[0.3036 1 0.3575] Add Capture UI To View
      (bind _returnvalue_2 (Game|ConstructObjectfromClass "/Game/UI/WBP_CaptureUI.WBP_CaptureUI_C"))
      (bind _output_get (Variables|Capture|SetCaptureWidget _returnvalue_2))
      (UserInterface|Viewport|AddtoViewport _output_get 0)
      ;[0.2654 0.6881 1] Add Dialogue UI to View
      (bind _returnvalue_3 (UserInterface|CreateWidget "/Game/UI/WBP_Dialogue.WBP_Dialogue_C"))
      (bind _output_get_2 (Variables|Default|SetDialogueWidget _returnvalue_3))
      (Variables|/Script/UMG.Widget|SetRenderOpacity (Variables|/Game/UI/WBP_Dialogue.WBP_Dialogue_C|GetParentOverlayBlock _output_get_2) 0.0)
      (UserInterface|Viewport|AddtoViewport _output_get_2 0)
      (bind _outactors (Actor|GetAllActorswithInterface "/Game/Blueprints/Interfaces/BPI_InteractableObject.BPI_InteractableObject_C"))
      (for _array_element _outactors
        (Class|BPIInteractableObject|SetupDialogueWidget(Message) _array_element (Variables|Default|GetDialogueWidget))
        ;[1 0.1236 0.1004] Create Captured Locations Array
        (bind _outactors_2 (Actor|GetAllActorsOfClass "/Game/Blueprints/BP_CapturedLocation.BP_CapturedLocation_C"))
        (for _array_element_2 _outactors_2
          (Utilities|Array|Add (Variables|Default|GetCapturedLocations) _array_element_2))
        (bind _returnvalue_4 (Game|ConstructObjectfromClass "/Game/UI/WBP_FadeScreen.WBP_FadeScreen_C"))
        (bind _output_get_3 (Variables|Ending|SetFadeScreen _returnvalue_4))
        (UserInterface|Viewport|AddtoViewport _output_get_3 0)))))

(fn ConstructionScript)

(fn FindAvailableCaptureLocation
  (for _array_element (Variables|Default|GetCapturedLocations)
    (if (not (Variables|/Game/Blueprints/BP_CapturedLocation.BP_CapturedLocation_C|GetIsOccupied _array_element))
      (Variables|/Game/Blueprints/BP_CapturedLocation.BP_CapturedLocation_C|SetIsOccupied _array_element true)
      (return _array_element))))

(fn ReleaseCaptureLocation
  (params (CaptureLocationToRelease :type BP%20Captured%20Location%20Object%20Reference))
  (Variables|/Game/Blueprints/BP_CapturedLocation.BP_CapturedLocation_C|SetIsOccupied CaptureLocationToRelease false)
  (return))