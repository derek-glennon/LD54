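; BP_Pillar is an interactable that moves the narrative from one room to another.
; Hovering shows a grab-hand cursor unless the narrative player controller is in capture mode.
; On interact, it locks input, runs timed leave and arrive calls on its two rooms, then updates CurrentRoom on the controller and all narrative characters.
; A flag triggers the ending-room event, and the top object's random-rotation logic is disconnected.
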(event Custom|OnBeginCursorOver_Event
  (params (TouchedActor :type Actor%20Object%20Reference))
  (if (not (Variables|/Game/Blueprints/BP_NarrativePlayerController.BP_NarrativePlayerController_C|GetInCaptureMode (Variables|Default|GetNarrativePlayerController)))
    (Variables|/Script/Engine.PlayerController|SetCurrentMouseCursor (Game|GetPlayerController 0) "GrabHand")))

(event Custom|OnEndCursorOver_Event
  (params (TouchedActor :type Actor%20Object%20Reference))
  (if (not (Variables|/Game/Blueprints/BP_NarrativePlayerController.BP_NarrativePlayerController_C|GetInCaptureMode (Variables|Default|GetNarrativePlayerController)))
    (Variables|/Script/Engine.PlayerController|SetCurrentMouseCursor (Game|GetPlayerController 0) "Default")))

(event EventBeginPlay
  (bind _asbp_narrative_player_controller (Utilities|Casting|CastToBP_NarrativePlayerController (Game|GetPlayerController 0)))
  (Variables|Default|SetNarrativePlayerController _asbp_narrative_player_controller)
  (EventDispatchers|BindEventtoOnBeginCursorOver (delegate Custom|OnBeginCursorOver_Event))
  (EventDispatchers|BindEventtoOnEndCursorOver (delegate Custom|OnEndCursorOver_Event)))

(event EventTick
  (params (DeltaSeconds :type Float%20%28single-precision%29)))

(event EventSetupDialogueWidget
  (params (DialogueWidget :type WBP%20Dialogue%20Object%20Reference))
  (Variables|Default|SetDialogueWidget DialogueWidget))

(event EventOnInteract
  (bind _narrativeplayercontroller (Variables|Default|GetNarrativePlayerController))
  (Input|DisableInput (Variables|Default|GetNarrativePlayerController) 0)
  (Variables|/Game/Blueprints/BP_NarrativePlayerController.BP_NarrativePlayerController_C|SetInTransition (Variables|Default|GetNarrativePlayerController) true)
  (Default|Leave (Variables|Default|GetLeavingRoom))
  (Utilities|FlowControl|Delay 1.0)
  (Default|Arrive (Variables|Default|GetArrivingRoom))
  (Utilities|FlowControl|Delay 1.5)
  (Input|EnableInput _narrativeplayercontroller _narrativeplayercontroller)
  (Variables|/Game/Blueprints/BP_NarrativePlayerController.BP_NarrativePlayerController_C|SetInTransition (Variables|Default|GetNarrativePlayerController) false)
  (Variables|/Game/Blueprints/BP_NarrativePlayerController.BP_NarrativePlayerController_C|SetCurrentRoom (Variables|Default|GetNarrativePlayerController) (Variables|Default|GetArrivingRoom))
  (bind _outactors (Actor|GetAllActorsOfClass "/Game/Characters/BP_NarrativeCharacter.BP_NarrativeCharacter_C"))
  (for _array_element _outactors
    (Variables|/Game/Characters/BP_NarrativeCharacter.BP_NarrativeCharacter_C|SetCurrentRoom _array_element (Variables|Default|GetArrivingRoom)))
  (if (Variables|Default|GetMovesToEndingRoom)
    (Default|OnEndingRoomArrived (Variables|Default|GetNarrativePlayerController))))

(fn ConstructionScript)