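; BP_FadeScreen is an actor that fades the view to black or back into the game through a screen mesh.
; BeginPlay creates a dynamic material on the mesh and caches the narrative player controller.
; Two timeline-driven events remap their lerp value through float curves into the material's FadeValue parameter.
; When the fade to black finishes, it calls ResetGameLoop on the controller, restarting the game loop.
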(event Custom|FadeToBlack
  (bind _lerpvalue (Timeline|ToBlack PlayFromStart)
    (:Update
      (Rendering|Material|SetScalarParameterValue (Variables|Default|GetDynamicMaterial) "FadeValue" (Math|Curves|GetFloatValue (Variables|Default|GetFadeToBlackCurve) _lerpvalue) :!class /Script/Engine.MaterialInstanceDynamic))
    (:Finished
      (Default|ResetGameLoop (Variables|Default|GetNarrativePlayerController)))))

(event Custom|FadeInToGame
  (bind _lerpvalue (Timeline|Timeline PlayFromStart)
    (:Update
      (Rendering|Material|SetScalarParameterValue (Variables|Default|GetDynamicMaterial) "FadeValue" (Math|Curves|GetFloatValue (Variables|Default|GetFadeInToGameCurve) _lerpvalue) :!class /Script/Engine.MaterialInstanceDynamic))))

(event EventBeginPlay
  (bind _returnvalue (Rendering|Material|CreateDynamicMaterialInstance (Variables|Default|GetFadeScreenMesh) 0 0 "None" :!class /Script/Engine.PrimitiveComponent))
  (Variables|Default|SetDynamicMaterial _returnvalue)
  (bind _asbp_narrative_player_controller (Utilities|Casting|CastToBP_NarrativePlayerController (Game|GetPlayerController 0)))
  (Variables|Default|SetNarrativePlayerController _asbp_narrative_player_controller))

(event Collision|EventActorBeginOverlap
  (params (OtherActor :type Actor%20Object%20Reference)))

(event EventTick
  (params (DeltaSeconds :type Float%20%28single-precision%29)))

(fn ConstructionScript)