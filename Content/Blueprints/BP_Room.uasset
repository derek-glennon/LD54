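; BP_Room is a room actor that animates itself moving in and out of place for a narrative game.
; On BeginPlay, the starting room registers itself as current room on the narrative player controller and every BP_NarrativeCharacter.
; Leave and Arrive teleport it to a start point, then timelines move it along curve-shaped lerps between arriving, main and leaving points.
; Once arrival finishes, all narrative characters reset their home transforms.
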(event Custom|Leave
  (Transformation|SetActorLocation (Transformation|GetActorLocation (Variables|Default|GetMainPoint)) false true)
  (bind _lerpvalue (Timeline|Main_To_Leaving PlayFromStart)
    (:Update
      (Transformation|SetActorLocation (Math|Interpolation|Ease "Linear" (Math|Curves|GetFloatValue (Variables|Default|GetMainToLeavingCurve) _lerpvalue) (Transformation|GetActorLocation (Variables|Default|GetMainPoint)) (Transformation|GetActorLocation (Variables|Default|GetLeavingPoint))) false false))))

(event Custom|Arrive
  (Transformation|SetActorLocation (Transformation|GetActorLocation (Variables|Default|GetArrivingPoint)) false true)
  (bind _lerpvalue (Timeline|Arriving_To_Main PlayFromStart)
    (:Update
      (Transformation|SetActorLocation (Math|Interpolation|Ease "Linear" (Math|Curves|GetFloatValue (Variables|Default|GetArrivingToMainCurve) _lerpvalue) (Transformation|GetActorLocation (Variables|Default|GetArrivingPoint)) (Transformation|GetActorLocation (Variables|Default|GetMainPoint))) false false))
    (:Finished
      (bind _outactors (Actor|GetAllActorsOfClass "/Game/Characters/BP_NarrativeCharacter.BP_NarrativeCharacter_C"))
      (for _array_element _outactors
        (Default|ResetHomeTransform _array_element)))))

(event EventBeginPlay
  (bind _asbp_narrative_player_controller (Utilities|Casting|CastToBP_NarrativePlayerController (Game|GetPlayerController 0)))
  (Variables|Default|SetNarrativePlayerController _asbp_narrative_player_controller)
  (if (Variables|Default|GetIsStartingRoom)
    (Variables|/Game/Blueprints/BP_NarrativePlayerController.BP_NarrativePlayerController_C|SetCurrentRoom (Variables|Default|GetNarrativePlayerController) self)
    (bind _outactors (Actor|GetAllActorsOfClass "/Game/Characters/BP_NarrativeCharacter.BP_NarrativeCharacter_C"))
    (for _array_element _outactors
      (Variables|/Game/Characters/BP_NarrativeCharacter.BP_NarrativeCharacter_C|SetCurrentRoom _array_element self))))

(event EventTick
  (params (DeltaSeconds :type Float%20%28single-precision%29)))

(fn ConstructionScript)