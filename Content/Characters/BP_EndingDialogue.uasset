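; BP_EndingDialogue is a dialogue character Blueprint that selects the lines for the game's ending.
; On interact, it swaps in repeat-ending dialogue if any lives have been created, with blob-specific lines taking priority when the ending character is a BP_Blob, then defers to the parent.
; Finishing talk re-triggers interaction after a short delay, and a specific emote re-enables player controller input.
; A fade-to-black call is left unconnected.
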(event EventBeginPlay
  (|CallParentFunction) ; This node is disabled and will not be called.\nDrag off pins to build functionality.
)

(event Collision|EventActorBeginOverlap
  (params (OtherActor :type Actor%20Object%20Reference)))

(event EventOnEmote
  (params (EmoteInteger :type Integer))
  (bind _narrativeplayercontroller (Variables|Default|GetNarrativePlayerController))
  (if (== EmoteInteger 1)
    (Input|EnableInput _narrativeplayercontroller _narrativeplayercontroller)))

(event EventOnTalkDone
  (Utilities|FlowControl|Delay 1.0)
  (CallFunction|OnInteract))

(event EventOnInteract
  (if (> (Variables|/Game/Blueprints/BP_NarrativePlayerController.BP_NarrativePlayerController_C|GetLivesCreated (Variables|Default|GetNarrativePlayerController)) 0)
    (Utilities|Array|Clear (Variables|Default|GetEndingDialogueArray))
    (Variables|Default|SetEndingDialogueArray (Variables|Dialogue|GetRepeatEndingsDialogue)))
  (Utilities|Casting|CastToBP_Blob (Variables|/Game/Blueprints/BP_NarrativePlayerController.BP_NarrativePlayerController_C|GetEndingCharacter (Variables|Default|GetNarrativePlayerController))
    (:then
      (Utilities|Array|Clear (Variables|Default|GetEndingDialogueArray))
      (Variables|Default|SetEndingDialogueArray (Variables|Dialogue|GetEndingBlobArray)))
    (:CastFailed
      _))
  (|CallParentFunction))

(fn ConstructionScript
  (|CallParentFunction))